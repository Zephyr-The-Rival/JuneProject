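; Game Instance Blueprint that handles hosting multiplayer sessions and joining them through invites.
; CreateSession creates an Advanced Session tagged with a SessionName property, then server-travels to LevelToTravelTo as a listen server.
; FixLevelPath builds the travel URL by trimming the level's soft object path at the last dot and appending "?listen".
; Accepted invites call JoinSession directly, with results reported only through debug prints.
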(event `CreateSession`
  (params (SessionName :type String))
  (`KismetSystemLibrary.PrintString` "CreatingSession...")
  (`CreateSessionCallbackProxyAdvanced.CreateAdvancedSession` (`|MakeArray` (`AdvancedSessionsLibrary.MakeLiteralSessionPropertyString` "SessionName" SessionName)) (`GameplayStatics.GetPlayerController` 0)
    (:`OnSuccess`
      (`KismetSystemLibrary.PrintString` "Creating Session Succeded \nServerTravel...")
      (bind _servertravelurl (`self.FixLevelPath` (`self.LevelToTravelTo`)))
      (`AdvancedSessionsLibrary.ServerTravel` _servertravelurl true) ; /Game/...?listen
      (`KismetSystemLibrary.PrintString` "Dont forget to set input mode to game only"))
    (:`OnFailure`
      (`KismetSystemLibrary.PrintString` "Creating Advanced Session failed"))))

(event `self.OnSessionInviteAccepted`
  (params (LocalPlayerNum :type Integer) (PersonInvited :type "BPUniqueNetId Structure") (SessionToJoin :type "BlueprintSessionResult Structure (by ref)"))
  (`JoinSessionCallbackProxy.JoinSession` (`GameplayStatics.GetPlayerController` 0) SessionToJoin
    (:`then`
      (`KismetSystemLibrary.PrintString` "Join via invite"))
    (:`OnSuccess`
      (`KismetSystemLibrary.PrintString` "Join seession via invite  succeeded"))
    (:`OnFailure`
      (`KismetSystemLibrary.PrintString` "Join seession via invite  failed"))))

(fn `FixLevelPath`
  (params (Level :type "World Soft Object Reference"))
  (returns (ServerTravelURL :type String))
  (locals (LocalPath :type String))
  (bind _localpath (`local.LocalPath`))
  (`|ExecutionSequence`
    (:`then_0`
      (set `local.LocalPath` (`KismetSystemLibrary.BreakSoftObjectPath` (`KismetSystemLibrary.Conv_SoftObjRefToSoftObjPath` Level))))
    (:`then_1`
      (set `local.LocalPath` (`KismetStringLibrary.GetSubstring` _localpath 0 (`KismetStringLibrary.FindSubstring` _localpath "." false true))))
    (:`then_2`
      (set `local.LocalPath` (`KismetStringLibrary.Concat_StrStr` (`local.LocalPath`) "?listen")))
    (:`then_3`
      (return (`local.LocalPath`)))))