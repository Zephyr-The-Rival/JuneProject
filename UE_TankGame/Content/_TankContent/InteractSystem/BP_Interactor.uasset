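; BP_Interactor is a component that detects the BP_Interactable its owner is looking at.
; It caches the owner's camera on BeginPlay, then line-traces forward from it every tick within InteractorRange.
; A new interactable hit is stored and broadcast with its prompt text.
; A trace with no hit clears it and broadcasts hover end every tick, while hitting a non-interactable leaves the previous hover in place.
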(event `self.ReceiveBeginPlay`
  (bind _returnvalue (`Actor.GetComponentByClass` (`self.GetOwner`) "/Script/Engine.CameraComponent"))
  (`/Engine/EditorBlueprintResources/StandardMacros.IsValid` _returnvalue
    (:`Is Valid`
      (set `self.PlayerCamrea` _returnvalue))))

(event `self.ReceiveTick`
  (params (DeltaSeconds :type "Float (single-precision)"))
  (bind _playercamrea (`self.PlayerCamrea`))
  (bind _returnvalue (`SceneComponent.K2_GetComponentLocation` _playercamrea))
  (bind _outhit (`KismetSystemLibrary.LineTraceSingle` _returnvalue (+ _returnvalue (* (`SceneComponent.GetForwardVector` _playercamrea) (`self.InteractorRange`))) "TraceTypeQuery3"))
  (bind (_bblockinghit _binitialoverlap _time _distance _location _impactpoint _normal _impactnormal _physmat _hitactor) (`GameplayStatics.BreakHitResult` _outhit))
  (if _bblockinghit
    (bind _asbp_interactable (cast `/Game/_TankContent/InteractSystem/BP_Interactable` _hitactor))
    (if (!= (`self.HoveredInteractale`) _asbp_interactable)
      (`self.HoveredNewInteractable` _asbp_interactable))
    (else
      (`self.NoInteractableFound`))))

(event `HoveredNewInteractable`
  (params (HoveredInteractale :type "/Game/_TankContent/InteractSystem/BP_Interactable Object Reference"))
  (bind _output_get (set `self.HoveredInteractale` HoveredInteractale))
  (`self.OnNewInteractableHovered` _output_get (`/Game/_TankContent/InteractSystem/BP_Interactable.GetInteractPrompText` _output_get)))

(event `NoInteractableFound`
  (set `self.HoveredInteractale` null)
  (`self.OnInteractableHoveredEnd`))